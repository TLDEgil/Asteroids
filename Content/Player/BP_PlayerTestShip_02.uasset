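; BP_PlayerTestShip_02 is a test player ship with four wings (top, bottom, left, right) that pivot to a shared sweep angle.
; BeginPlay sets the angle range and sweep alpha.
; Each Tick lerps that range by the alpha and applies the mirrored result to the wing attach points, pitch for top and bottom, yaw for left and right.
; Nothing here changes the sweep afterwards, so the wings hold at the maximum angle.
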(event EventBeginPlay
  (Variables|Default|SetWingAngleMin 0.0)
  (Variables|Default|SetWingAngleMax 5e+01)
  (Variables|Default|SetWingSweep 1.0))

(event Collision|EventActorBeginOverlap
  (params (OtherActor :type Actor%20Object%20Reference)))

(event EventTick
  (params (DeltaSeconds :type Float%20%28single-precision%29))
  (bind _topwingattachpoint (Variables|Default|GetTopWingAttachPoint))
  (bind _winganglemin (Variables|Default|GetWingAngleMin))
  (bind _winganglemax (Variables|Default|GetWingAngleMax))
  (bind _wingsweep (Variables|Default|GetWingSweep))
  (bind _bottomwingattachpoint (Variables|Default|GetBottomWingAttachPoint))
  (bind _leftwingattachpoint (Variables|Default|GetLeftWingAttachPoint))
  (bind _rightwingattachpoint (Variables|Default|GetRightWingAttachPoint))
  (bind _returnvalue (Math|Float|Lerp _winganglemin _winganglemax _wingsweep))
  (bind _relativerotation (Variables|/Script/Engine.SceneComponent|GetRelativeRotation _topwingattachpoint))
  (bind _relativerotation_2 (Variables|/Script/Engine.SceneComponent|GetRelativeRotation _leftwingattachpoint))
  (bind _relativerotation_3 (Variables|/Script/Engine.SceneComponent|GetRelativeRotation _rightwingattachpoint))
  (bind _relativerotation_4 (Variables|/Script/Engine.SceneComponent|GetRelativeRotation _bottomwingattachpoint))
  (Transformation|SetRelativeRotation _topwingattachpoint (Math|Rotator|MakeRotator (.roll _relativerotation) (- 0.0 _returnvalue) (.yaw _relativerotation)) false false)
  (Transformation|SetRelativeRotation _bottomwingattachpoint (Math|Rotator|MakeRotator (.roll _relativerotation_4) _returnvalue (.yaw _relativerotation_4)) false false)
  (Transformation|SetRelativeRotation _leftwingattachpoint (Math|Rotator|MakeRotator (.roll _relativerotation_2) (.pitch _relativerotation_2) _returnvalue) false false)
  (Transformation|SetRelativeRotation _rightwingattachpoint (Math|Rotator|MakeRotator (.roll _relativerotation_3) (.pitch _relativerotation_3) (- 0.0 _returnvalue)) false false))

(fn ConstructionScript)